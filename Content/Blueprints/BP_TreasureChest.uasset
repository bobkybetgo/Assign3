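; BP_TreasureChest is an actor whose cube changes to a random color when it receives a trace-hit event.
; The Construction Script creates a dynamic material instance from M_Basic_Floor and applies the Color variable to it.
; The TraceHitActorwithComponent event creates a fresh instance on each call and sets its color from a random unit vector.
; No chest opening or loot logic is present.
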(event EventBeginPlay)

(event EventActorBeginOverlap
  (params (OtherActor :type Actor%20Object%20Reference)))

(event EventTick
  (params (DeltaSeconds :type Float%20%28single-precision%29)))

(event EventTraceHitActorwithComponent
  (params (Component :type Primitive%20Component%20Object%20Reference))
  (Utilities|FlowControl|Sequence
    (:then_0
      (bind _returnvalue (Rendering|Material|CreateDynamicMaterialInstance (Variables|Default|GetCube) 0 "/Game/StarterContent/Materials/M_Basic_Floor.M_Basic_Floor" :!class /Script/Engine.PrimitiveComponent))
      (Variables|Default|SetMaterial _returnvalue)
      (Rendering|Material|SetVectorParameterValue (Variables|Default|GetMaterial) "Color" (Math|Conversions|ToLinearColor(Vector) (Math|Random|RandomUnitVector)) :!class /Script/Engine.MaterialInstanceDynamic))))

(fn ConstructionScript
  (Utilities|FlowControl|Sequence
    (:then_0
      (bind _returnvalue (Rendering|Material|CreateDynamicMaterialInstance (Variables|Default|GetCube) 0 "/Game/StarterContent/Materials/M_Basic_Floor.M_Basic_Floor" :!class /Script/Engine.PrimitiveComponent))
      (Variables|Default|SetMaterial _returnvalue)
      (Rendering|Material|SetVectorParameterValue (Variables|Default|GetMaterial) "Color" (Variables|Default|GetColor) :!class /Script/Engine.MaterialInstanceDynamic))))